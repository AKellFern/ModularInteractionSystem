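; BP_Door is an interactable door that swings open when unlocked and closes itself shortly afterwards.
; ExecuteInteraction updates the InteractableComponent's text, disables interaction and plays a timeline that rotates PivotPoint's yaw toward OpenYaw.
; After a short delay the timeline reverses, and interaction is re-enabled as closing begins.
; IsOpen gates the opening, but its only setter here is never run.
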(event `self.ExecuteInteraction`
  (params (InteractingActor :type "Actor Object Reference"))
  (if (`self.bIsUnlocked`)
    (set `InteractableComponent.InteractionText` "Open Door" (`self.InteractableComponent`))
    (if (not (`self.bIsOpen`))
      (set `InteractableComponent.bCanInteract` false (`self.InteractableComponent`))
      (bind (_direction _alpha) (`Timeline|TL_DoorOpen`)
        (:`Update`
          (`SceneComponent.K2_SetRelativeRotation` (`self.Pivot Point`) (`KismetMathLibrary.MakeRotator` 0.0 0.0 (`KismetMathLibrary.Lerp` 0.0 (`self.openYaw`) _alpha)) false false))
        (:`Finished`
          (if (`|EnumEquality` _direction "Forward")
            (`KismetSystemLibrary.Delay` 1.0)
            (`TimelineComponent.Reverse` (`self.TL_DoorOpen`))
            (set `InteractableComponent.bCanInteract` true (`self.InteractableComponent`))))))))

(fn `UserConstructionScript`)