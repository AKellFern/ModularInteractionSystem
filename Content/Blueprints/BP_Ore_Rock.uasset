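; BP_Ore_Rock is a mineable ore rock placed in the world as copper, gold, iron, silver or tin.
; The construction script switches on OreType to set the mesh, a material (each type at a different slot index) and the InteractableComponent prompt.
; ExecuteInteraction prints an "Added to Inventory" message and destroys the actor, with no actual inventory update in this Blueprint.
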(event `self.ExecuteInteraction`
  (params (InteractingActor :type "Actor Object Reference"))
  (`KismetSystemLibrary.PrintString` (`KismetTextLibrary.Conv_TextToString` (`|FormatText` "Added {OreType} Ore to Inventory" (`|GetEnumeratorNameAsString` (`self.OreType`)))))
  (`self.K2_DestroyActor`))

(fn `UserConstructionScript`
  (bind _cube (`self.Cube`))
  (bind _cube_2 (`self.Cube`))
  (bind _cube_3 (`self.Cube`))
  (bind _cube_4 (`self.Cube`))
  (bind _cube_5 (`self.Cube`))
  (`parent.UserConstructionScript`)
  (switch `/Game/Assets/OreRocks/E_OreType` (`self.OreType`)
    (:`NewEnumerator0`
      ; Copper Selection
      (`StaticMeshComponent.SetStaticMesh` _cube_3 "/Game/Assets/OreRocks/Mesh/Copper/SM_CopperOre.SM_CopperOre")
      (`PrimitiveComponent.SetMaterial` _cube_3 0 "/Game/Assets/OreRocks/Material/MI_Ore_Copper.MI_Ore_Copper")
      (set `InteractableComponent.InteractionText` "Mine Copper" (`self.InteractableComponent`)))
    (:`NewEnumerator1`
      ; Gold Selection
      (`StaticMeshComponent.SetStaticMesh` _cube_4 "/Game/Assets/OreRocks/Mesh/Gold/SM_GoldenOre.SM_GoldenOre")
      (`PrimitiveComponent.SetMaterial` _cube_4 1 "/Game/Assets/OreRocks/Material/MI_Ore_Gold.MI_Ore_Gold")
      (set `InteractableComponent.InteractionText` "Mine Gold" (`self.InteractableComponent`)))
    (:`NewEnumerator2`
      ; Iron Selction
      (`StaticMeshComponent.SetStaticMesh` _cube_5 "/Game/Assets/OreRocks/Mesh/Iron/SM_IronOre.SM_IronOre")
      (`PrimitiveComponent.SetMaterial` _cube_5 2 "/Game/Assets/OreRocks/Material/MI_Ore_Iron.MI_Ore_Iron")
      (set `InteractableComponent.InteractionText` "Mine Iron" (`self.InteractableComponent`)))
    (:`NewEnumerator3`
      ; Silver Selection
      (`StaticMeshComponent.SetStaticMesh` _cube "/Game/Assets/OreRocks/Mesh/Silver/SM_SilverOre.SM_SilverOre")
      (`PrimitiveComponent.SetMaterial` _cube 3 "/Game/Assets/OreRocks/Material/MI_Ore_Silver.MI_Ore_Silver")
      (set `InteractableComponent.InteractionText` "Mine Silver" (`self.InteractableComponent`)))
    (:`NewEnumerator4`
      ; Tin Selection
      (`StaticMeshComponent.SetStaticMesh` _cube_2 "/Game/Assets/OreRocks/Mesh/Tin/SM_TinOre.SM_TinOre")
      (`PrimitiveComponent.SetMaterial` _cube_2 4 "/Game/Assets/OreRocks/Material/MI_Ore_Tin.MI_Ore_Tin")
      (set `InteractableComponent.InteractionText` "Mine Tin" (`self.InteractableComponent`)))))