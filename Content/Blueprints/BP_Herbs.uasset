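; Gatherable herb actor whose HerbType enum selects one of five herbs: mint, sage, rosemary, thyme or chamomile.
; The construction script switches on HerbType to set the mesh, the InteractableComponent prompt and the shared MI_Plants material, using a different slot index per herb.
; ExecuteInteraction only prints an "Added to Inventory" message and destroys the actor; no inventory is actually updated here.
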(event `self.ExecuteInteraction`
  (params (InteractingActor :type "Actor Object Reference"))
  (`KismetSystemLibrary.PrintString` (`KismetTextLibrary.Conv_TextToString` (`|FormatText` "Added {HerbType} to Inventory" (`|GetEnumeratorNameAsString` (`self.HerbType`)))))
  (`self.K2_DestroyActor`))

(fn `UserConstructionScript`
  (bind _cube (`self.Cube`))
  (bind _cube_2 (`self.Cube`))
  (bind _cube_3 (`self.Cube`))
  (bind _cube_4 (`self.Cube`))
  (bind _cube_5 (`self.Cube`))
  (`parent.UserConstructionScript`)
  (switch `/Game/Assets/Herbs/E_HerbType` (`self.HerbType`)
    (:`NewEnumerator0`
      ; Mint Selection
      (`StaticMeshComponent.SetStaticMesh` _cube_3 "/Game/Assets/Herbs/SM_Mint.SM_Mint")
      (`PrimitiveComponent.SetMaterial` _cube_3 0 "/Game/Assets/Herbs/MI_Plants.MI_Plants")
      (set `InteractableComponent.InteractionText` "Gather Mint" (`self.InteractableComponent`)))
    (:`NewEnumerator1`
      ; Sage Selection
      (`StaticMeshComponent.SetStaticMesh` _cube_4 "/Game/Assets/Herbs/SM_Sage.SM_Sage")
      (`PrimitiveComponent.SetMaterial` _cube_4 1 "/Game/Assets/Herbs/MI_Plants.MI_Plants")
      (set `InteractableComponent.InteractionText` "Gather Sage" (`self.InteractableComponent`)))
    (:`NewEnumerator2`
      ; Rosemary Selction
      (`StaticMeshComponent.SetStaticMesh` _cube_5 "/Game/Assets/Herbs/SM_Rosemary.SM_Rosemary")
      (`PrimitiveComponent.SetMaterial` _cube_5 2 "/Game/Assets/Herbs/MI_Plants.MI_Plants")
      (set `InteractableComponent.InteractionText` "Gather Rosemary" (`self.InteractableComponent`)))
    (:`NewEnumerator3`
      ; Thyme Selection
      (`StaticMeshComponent.SetStaticMesh` _cube "/Game/Assets/Herbs/SM_Thyme.SM_Thyme")
      (`PrimitiveComponent.SetMaterial` _cube 3 "/Game/Assets/Herbs/MI_Plants.MI_Plants")
      (set `InteractableComponent.InteractionText` "Gather Thyme" (`self.InteractableComponent`)))
    (:`NewEnumerator4`
      ; Chamomille Selection
      (`StaticMeshComponent.SetStaticMesh` _cube_2 "/Game/Assets/Herbs/SM_Chamomille.SM_Chamomille")
      (`PrimitiveComponent.SetMaterial` _cube_2 4 "/Game/Assets/Herbs/MI_Plants.MI_Plants")
      (set `InteractableComponent.InteractionText` "Gather Chamomille" (`self.InteractableComponent`)))))