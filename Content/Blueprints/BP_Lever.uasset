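; BP_Lever is an interactable lever that unlocks a referenced door.
; On interaction it sets the door's IsUnlocked flag and changes the interaction prompt to show the door is unlocked.
; A timeline then lerps the lever mesh's roll from its locked angle to its unlocked angle.
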(event `self.ExecuteInteraction`
  (params (InteractingActor :type "Actor Object Reference"))
  (set `/Game/Blueprints/BP_Door.bIsUnlocked` true (`self.DoorRef`))
  (set `self.StartRoll` (`self.LockedRoll`))
  (set `self.TargetRoll` (`self.UnlockedRoll`))
  (set `InteractableComponent.InteractionText` "Door is unlocked" (`self.InteractableComponent`))
  (bind (_direction _alpha) (`Timeline|Timeline`)
    (:`Update`
      (`SceneComponent.K2_SetRelativeRotation` (`self.SM_Lever_4`) (`KismetMathLibrary.MakeRotator` (`KismetMathLibrary.Lerp` (`self.StartRoll`) (`self.TargetRoll`) _alpha)) false false))))

(fn `UserConstructionScript`)